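; OceanSimulator is a Blueprint that feeds ocean configuration into the MPC_Ocean material parameter collection when play begins.
; It copies displacement map size and wind direction from SpectrumConfig, along with its own patch length and displacement factor.
; It also writes the negated forward vector of the Sun actor as the sunlight direction.
; All values are set once at BeginPlay, and the Blueprint graphs contain no wave simulation logic.
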(event EventBeginPlay
  (bind _spectrumconfig (Variables|Default|GetSpectrumConfig))
  (bind (_dispmapdimension _patchlength _winddirection) (Utilities|Struct|BreakSpectrumData _spectrumconfig))
  (bind (_x _y) (Math|Vector2D|BreakVector2D _winddirection))
  (Rendering|Material|SetScalarParameterValue "/Game/APiratesLife/Materials/MPC_Ocean.MPC_Ocean" "DisplacementMapDimensions" (Math|Conversions|ToFloat(Integer) _dispmapdimension) :!class /Script/Engine.KismetMaterialLibrary)
  (Rendering|Material|SetScalarParameterValue "/Game/APiratesLife/Materials/MPC_Ocean.MPC_Ocean" "PatchLength" (Variables|Default|GetMaterialPatchLength) :!class /Script/Engine.KismetMaterialLibrary)
  (Rendering|Material|SetVectorParameterValue "/Game/APiratesLife/Materials/MPC_Ocean.MPC_Ocean" "WindDirection" (Utilities|Struct|MakeLinearColor _x _y 0.0 0.0) :!class /Script/Engine.KismetMaterialLibrary)
  (Rendering|Material|SetScalarParameterValue "/Game/APiratesLife/Materials/MPC_Ocean.MPC_Ocean" "DisplacementFactor" (Variables|Default|GetMaterialDisplacementFactor) :!class /Script/Engine.KismetMaterialLibrary)
  (Rendering|Material|SetVectorParameterValue "/Game/APiratesLife/Materials/MPC_Ocean.MPC_Ocean" "SunLightDirection" (Math|Conversions|ToLinearColor(Vector) (Math|Vector|NegateVector (Transformation|GetActorForwardVector (Variables|Default|GetSun)))) :!class /Script/Engine.KismetMaterialLibrary))

(event Collision|EventActorBeginOverlap
  (params (OtherActor :type Actor%20Object%20Reference)))

(fn ConstructionScript)